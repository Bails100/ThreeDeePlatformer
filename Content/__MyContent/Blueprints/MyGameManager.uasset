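; MyGameManager is a game manager Blueprint that tracks the game state (Running, Win, Lose, Abandon) and drives the matching UI and pause behavior.
; Init has the game mode create the UI, initializes the player, then enters Running.
; SetState hides the UI on a change, then either shows the health HUD and unpauses, or shows the result widget with the mouse and pauses.
; ResetGame moves the player to the first PlayerStart and reinitializes it.
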(fn `Get State`
  (returns (State :type "/Game/__MyContent/Blueprints/E_MyGameStates Enum"))
  (return (`self.Current Game State`)))

(fn `Init`
  (bind _asgame_mode (cast `/Game/__MyContent/Blueprints/Game_Mode` (`GameplayStatics.GetGameMode`)))
  (`/Game/__MyContent/Blueprints/Game_Mode.Creat UI` _asgame_mode)
  (`/Game/ThirdPersonBP/Blueprints/ThirdPersonCharacter.Init` (`self.My Player`))
  (`self.Set State` "NewEnumerator0"))

(fn `Reset game`
  (bind _my_player (`self.My Player`))
  (bind _outactors (`GameplayStatics.GetAllActorsOfClass` "/Script/Engine.PlayerStart"))
  (`self.K2_SetActorLocation` _my_player (`self.K2_GetActorLocation` (`|GetArrayItem` _outactors)) false false)
  ;[1 1 1] Add Player Init funtion here
  (`/Game/ThirdPersonBP/Blueprints/ThirdPersonCharacter.Init` _my_player))

(fn `Set State`
  (params (`New state` :type "/Game/__MyContent/Blueprints/E_MyGameStates Enum" :default "NewEnumerator0"))
  (if (`|EnumInequality` `New state` (`self.Current Game State`))
    (`/Game/__MyContent/Blueprints/Function_Library.Hide UI`)
    (bind _output_get (set `self.Current Game State` `New state`))
    (switch `/Game/__MyContent/Blueprints/E_MyGameStates` _output_get
      (:`NewEnumerator0`
        (`/Game/__MyContent/Blueprints/Function_Library.Show Mouse` false)
        (`GameplayStatics.SetGamePaused` false)
        (`self.Show Hud` true))
      (:`NewEnumerator1`
        (`Widget.SetVisibility` (`self.Widget_win`) "Visible")
        (`/Game/__MyContent/Blueprints/Function_Library.Show Mouse` true :!label _label)
        (`GameplayStatics.SetGamePaused` true))
      (:`NewEnumerator2`
        (`Widget.SetVisibility` (`self.Widget_Lose`) "Visible")
        (goto _label))
      (:`NewEnumerator3`
        (`Widget.SetVisibility` (`self.Widget_Abandon`) "Visible")
        (goto _label)))))

(fn `Show Hud`
  (params (Visible :type Boolean))
  (bind _widget_health (`self.Widget_Health`))
  (if Visible
    (`Widget.SetVisibility` _widget_health "Visible")
    (else
      (`Widget.SetVisibility` _widget_health "Hidden"))))

(fn `UserConstructionScript`)