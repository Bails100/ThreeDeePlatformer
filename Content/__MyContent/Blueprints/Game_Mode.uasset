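; Game mode Blueprint that holds a reference to the game manager and provides setup for the game's UI.
; On BeginPlay it caches the first MyGameManager actor found in the level.
; CreatUI, not called within this file, creates the Abandon, Win, Lose and Health widgets, stores each on the manager returned by GetMyGAmeManger and adds them all to the viewport.
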(event `self.ReceiveBeginPlay`
  (bind _outactors (`GameplayStatics.GetAllActorsOfClass` "/Game/__MyContent/Blueprints/MyGameManager.MyGameManager_C"))
  (set `self.My Game Manager` (`|GetArrayItem` _outactors)))

(fn `Creat UI`
  (bind _my_game_manager (`/Game/__MyContent/Blueprints/Function_Library.Get My GAme manger`))
  (bind _returnvalue (`|CreateWidget` "/Game/__MyContent/UI/Widget_Abandon.Widget_Abandon_C"))
  (bind _output_get (set `/Game/__MyContent/Blueprints/MyGameManager.Widget_Abandon` _returnvalue _my_game_manager))
  (`UserWidget.AddToViewport` _output_get 0)
  (bind _returnvalue_2 (`|CreateWidget` "/Game/__MyContent/UI/Widget_Win.Widget_Win_C"))
  (bind _output_get_2 (set `/Game/__MyContent/Blueprints/MyGameManager.Widget_win` _returnvalue_2 _my_game_manager))
  (`UserWidget.AddToViewport` _output_get_2 0)
  (bind _returnvalue_3 (`|CreateWidget` "/Game/__MyContent/UI/Widget_Lose.Widget_Lose_C"))
  (bind _output_get_3 (set `/Game/__MyContent/Blueprints/MyGameManager.Widget_Lose` _returnvalue_3 _my_game_manager))
  (`UserWidget.AddToViewport` _output_get_3 0)
  (bind _returnvalue_4 (`|CreateWidget` "/Game/__MyContent/UI/Widget_Health.Widget_Health_C"))
  (bind _output_get_4 (set `/Game/__MyContent/Blueprints/MyGameManager.Widget_Health` _returnvalue_4 _my_game_manager))
  (`UserWidget.AddToViewport` _output_get_4 0))

(fn `UserConstructionScript`)